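; BP_Bricks is a breakable brick that loses a life whenever a BP_Ball hits its cube.
; UpdateBrickColor sets the cube's material by remaining lives, running at construction and after each non-lethal hit.
; At zero lives the brick destroys itself, then counts remaining BP_Bricks actors.
; If none remain, it shows the WBP_Win widget, pauses the game and sets mouse cursor visibility from the pause result.
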(event OnComponentHit(Cube)
  (params (HitComponent :type Primitive%20Component%20Object%20Reference) (OtherActor :type Actor%20Object%20Reference) (OtherComp :type Primitive%20Component%20Object%20Reference) (NormalImpulse :type Vector :default "0, 0, 0") (Hit :type Hit%20Result%20Structure%20%28by%20ref%29))
  (Utilities|Casting|CastToBP_Ball OtherActor)
  (bind _result (Math|Integer|DecrementInt (Variables|Default|GetBrickLives))
    (:%20%20
      (if (== _result 0)
        (Actor|DestroyActor)
        (bind _outactors (Actor|GetAllActorsOfClass "BP_Bricks_C"))
        (if (== (Utilities|Array|Length _outactors) 0)
          (bind _returnvalue (UserInterface|CreateWidget "/Game/BP/Interface/WBP_Win.WBP_Win_C"))
          (UserInterface|Viewport|AddtoViewport _returnvalue 0)
          (bind _returnvalue_2 (Game|SetGamePaused true))
          (Variables|/Script/Engine.PlayerController|SetbShowMouseCursor (Game|GetPlayerController 0) _returnvalue_2))
        (else
          (CallFunction|UpdateBrickColor))))))

(event EventBeginPlay)

(fn ConstructionScript
  (CallFunction|UpdateBrickColor))

(fn UpdateBrickColor
  (bind _cube (Variables|Default|GetCube))
  (switch int (Variables|Default|GetBrickLives)
    (:1
      (Rendering|Material|SetMaterial _cube 0 0))
    (:2
      (Rendering|Material|SetMaterial _cube 0 0))
    (:3
      (Rendering|Material|SetMaterial _cube 0 0))))