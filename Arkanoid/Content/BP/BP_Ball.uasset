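; BP_Ball is the physics ball of a brick-breaker game, launched diagonally by an impulse on BeginPlay.
; Each hit raises its speed slightly up to a cap, clamps velocity to exactly that speed, and updates the paddle's HUD score for Brick-tagged actors.
; On destruction it respawns through BallPosition while the paddle has Shoots left, otherwise shows game over and pauses.
; A BallRotation event yaws its spring arm.
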(event Custom|BallRotation
  (params (Rotation :type Float%20%28double-precision%29))
  (Transformation|AddLocalRotation (Variables|Default|GetSpringArm) (Math|Rotator|MakeRotator 0.0 0.0 (* Rotation 0.8)) false false))

(event EventBeginPlay
  (bind _ballspeed (Variables|Default|GetBallSPeed))
  (bind _returnvalue (* _ballspeed 5e+01))
  (Physics|AddImpulse (Variables|Default|GetSphere) (Math|Vector|MakeVector _returnvalue _returnvalue 0.0) "None" false)
  (bind _asbp_paddle (Utilities|Casting|CastToBP_Paddle (Game|Player|GetPlayerPawn 0)))
  (Variables|Default|SetAs%20BP%20Paddle _asbp_paddle))

(event Collision|EventHit
  (params (MyComp :type Primitive%20Component%20Object%20Reference) (Other :type Actor%20Object%20Reference) (OtherComp :type Primitive%20Component%20Object%20Reference) (bSelfMoved :type Boolean) (HitLocation :type Vector :default "0, 0, 0") (HitNormal :type Vector :default "0, 0, 0") (NormalImpulse :type Vector :default "0, 0, 0") (Hit :type Hit%20Result%20Structure%20%28by%20ref%29))
  (if (> (* (Variables|Default|GetBallSPeed) 1.03) 2.6e+03)
    _
    (else
      (Variables|Default|SetBallSPeed (* (Variables|Default|GetBallSPeed) 1.03))))
  (bind _returnvalue (Physics|GetPhysicsLinearVelocity (Variables|Default|GetSphere) "None"))
  (Physics|SetPhysicsLinearVelocity (Variables|Default|GetSphere) (Math|Vector|ClampVectorSize _returnvalue (Variables|Default|GetBallSPeed) (Variables|Default|GetBallSPeed)) false "None")
  (if (Actor|ActorHasTag Other "Brick")
    (Default|UpdateScore (Variables|/Game/BP/BP_Paddle.BP_Paddle_C|GetPlayerHUD (Variables|Default|GetAs%20BP%20Paddle)))))

(event EventDestroyed
  (if (> (Variables|/Game/BP/BP_Paddle.BP_Paddle_C|GetShoots (Variables|Default|GetAs%20BP%20Paddle)) 0)
    (Default|SpawnBall (Variables|Default|GetBallPosition))
    (else
      (bind _returnvalue (UserInterface|CreateWidget "/Game/BP/Interface/WBP_GameOver.WBP_GameOver_C"))
      (UserInterface|Viewport|AddtoViewport _returnvalue 0)
      (bind _returnvalue_2 (Game|SetGamePaused true))
      (Variables|/Script/Engine.PlayerController|SetbShowMouseCursor (Game|GetPlayerController 0) _returnvalue_2))))

(fn ConstructionScript)