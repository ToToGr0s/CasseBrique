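; BP_Ball_Spawner is an actor that spawns a BP_Ball at its own transform when play begins.
; SpawnBall passes the spawner to the new ball as BallPosition and stores it as CurrentBall, which GetBall exposes.
; Before spawning, it also caches the first spawner and ball found in the level, though neither reference is used here.
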(event Custom|SpawnBall
  (bind _returnvalue (Actor|GetActorOfClass "BP_Ball_Spawner_C"))
  (Variables|Default|SetBP_BallSpawner _returnvalue)
  (bind _returnvalue_2 (Actor|GetActorOfClass "/Game/BP/Ball/BP_Ball.BP_Ball_C"))
  (Variables|Default|SetBP_Ball _returnvalue_2)
  (bind _returnvalue_3 (Game|SpawnActorfromClass "/Game/BP/Ball/BP_Ball.BP_Ball_C" (Transformation|GetActorTransform) "Undefined" "MultiplyWithRoot" 0 self 0))
  (Variables|Default|SetCurrent%20ball _returnvalue_3))

(event EventBeginPlay
  (CallFunction|SpawnBall))

(fn ConstructionScript)

(fn GetBall
  (return (Variables|Default|GetCurrent%20ball)))