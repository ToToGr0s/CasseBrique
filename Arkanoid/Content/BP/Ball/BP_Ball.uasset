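; BP_Ball is the ball in a paddle-and-brick game, with a rotatable camera for shooting ducks.
; An impulse launches it, and each hit raises its clamped speed up to a cap, with brick hits updating the paddle HUD score.
; PressedE line-traces from the scene capture to destroy ducks; clearing all advances the level or shows the win screen.
; On destruction it respawns while Shoots remain, otherwise shows game over.
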(event Custom|BallRotation
  (params (Rotation :type Float%20%28double-precision%29))
  ;[1 0 0 0.5] Camera ball position
  (Transformation|AddLocalRotation (Variables|Default|GetSpringArm) (Math|Rotator|MakeRotator 0.0 0.0 (* Rotation 0.8)) false false))

(event Custom|Pressed%20E
  (params (State :type Boolean))
  (bind _scenecapturecomponent2d (Variables|Default|GetSceneCaptureComponent2D))
  (bind _returnvalue (Transformation|GetWorldLocation _scenecapturecomponent2d))
  ;[0 0.9115 0.8204 0.5] Check Collsion with BP DUCK
  (if State
    (bind (_outhit _returnvalue_2) (Collision|LineTraceByChannel _returnvalue (+ (* (Math|Vector|GetForwardVector (Transformation|GetWorldRotation _scenecapturecomponent2d)) 5e+02) _returnvalue) "TraceTypeQuery1" true 0 "None"))
    ;[0.5972 0.9531 0 0.5] Get Duck Reminnig
    (if _returnvalue_2
      (bind _asbp_duck (Utilities|Casting|CastToBP_Duck (.HitActor (Collision|BreakHitResult _outhit))))
      (Audio|PlaySound2D "/Game/Sound/0212.0212" 1.0 1.0 0.0 0 0)
      (Utilities|FlowControl|Delay 0.6)
      (Actor|DestroyActor _asbp_duck)
      (CallFunction|GetDuckRemining))))

(event EventBeginPlay
  (bind _ballspeed (Variables|Default|GetBallSPeed))
  (bind _returnvalue (* _ballspeed 5e+01))
  ;[0 0.674 0.1576 0.5] Set ball velocity
  (Physics|AddImpulse (Variables|Default|GetSphere) (Math|Vector|MakeVector _returnvalue (* _returnvalue (Math|Random|RandomFloatinRange 1.0 -1.0)) 0.0) "None" false)
  (bind _asbp_paddle (Utilities|Casting|CastToBP_Paddle (Game|Player|GetPlayerPawn 0)))
  (Variables|Default|SetAs%20BP%20Paddle _asbp_paddle))

(event Collision|EventHit
  (params (MyComp :type Primitive%20Component%20Object%20Reference) (Other :type Actor%20Object%20Reference) (OtherComp :type Primitive%20Component%20Object%20Reference) (bSelfMoved :type Boolean) (HitLocation :type Vector :default "0, 0, 0") (HitNormal :type Vector :default "0, 0, 0") (NormalImpulse :type Vector :default "0, 0, 0") (Hit :type Hit%20Result%20Structure%20%28by%20ref%29))
  ;[0.749 0.6601 0.01314 0.5] Ball acceleration
  (if (> (* (Variables|Default|GetBallSPeed) 1.01) 2.4e+03)
    _
    (else
      (Variables|Default|SetBallSPeed (* (Variables|Default|GetBallSPeed) 1.01))))
  (bind _returnvalue (Physics|GetPhysicsLinearVelocity (Variables|Default|GetSphere) "None"))
  (Physics|SetPhysicsLinearVelocity (Variables|Default|GetSphere) (Math|Vector|ClampVectorSize _returnvalue (Variables|Default|GetBallSPeed) (Variables|Default|GetBallSPeed)) false "None")
  (if (Actor|ActorHasTag Other "Brick")
    (Default|UpdateScore (Variables|/Game/BP/OnMap/BP_Paddle.BP_Paddle_C|GetPlayerHUD (Variables|Default|GetAs%20BP%20Paddle)))))

(event EventDestroyed
  ;[0.002113 0.2763 0.6948 0.5] Check end game
  (if (> (Variables|/Game/BP/OnMap/BP_Paddle.BP_Paddle_C|GetShoots (Variables|Default|GetAs%20BP%20Paddle)) 0)
    (Default|SpawnBall (Variables|Default|GetBallPosition))
    (else
      (bind _returnvalue (UserInterface|CreateWidget "/Game/BP/Interface/WBP_GameOver.WBP_GameOver_C"))
      (UserInterface|Viewport|AddtoViewport _returnvalue 0)
      (bind _returnvalue_2 (Game|SetGamePaused true))
      (Variables|/Script/Engine.PlayerController|SetbShowMouseCursor (Game|GetPlayerController 0) _returnvalue_2))))

(fn ConstructionScript)

(fn GetDuckRemining
  (bind _outactors (Actor|GetAllActorsOfClass "/Game/BP/OnMap/BP_Duck.BP_Duck_C"))
  (if (== (Utilities|Array|Length _outactors) 0)
    (bind _returnvalue (Actor|GetActorOfClass "/Game/BP/OnMap/BP_LevelTracker.BP_LevelTracker_C"))
    (switch int (Variables|/Game/BP/OnMap/BP_LevelTracker.BP_LevelTracker_C|Getlevel _returnvalue)
      (:1
        (Game|OpenLevel(byObjectReference) "/Game/Maps/Level2.Level2"))
      (:2
        (Game|OpenLevel(byObjectReference) "/Game/Maps/Level3.Level3"))
      (:3
        (Game|OpenLevel(byObjectReference) "/Game/Maps/Level4.Level4"))
      (:4
        (Game|OpenLevel(byObjectReference) "/Game/Maps/Level5.Level5"))
      (:5
        (Game|OpenLevel(byObjectReference) "/Game/Maps/Level6.Level6"))
      (:6
        (bind _returnvalue_2 (UserInterface|CreateWidget "/Game/BP/Interface/WBP_Win.WBP_Win_C"))
        (UserInterface|Viewport|AddtoViewport _returnvalue_2 0)
        (bind _returnvalue_3 (Game|SetGamePaused true))
        (Variables|/Script/Engine.PlayerController|SetbShowMouseCursor (Game|GetPlayerController 0) _returnvalue_3)
        (Input|SetInputModeUIOnly 0 0 "DoNotLock" false)))))