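; BP_Paddle is the player-controlled paddle that moves, aims and interacts with the ball, and sets up the HUD.
; BeginPlay adds the Enhanced Input context and HUD, and move input slides the paddle along local Y with sweep.
; Look input finds BP_Ball and sends it an atan2-derived angle, while pick input forwards press and release to it.
; Pause input opens the pause widget, pauses the game and switches to UI-only input.
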(event Input|EnhancedActionEvents|EnhancedInputActionIA_Look
  (params (ActionValue :type Vector%202D%20Structure) (ElapsedSeconds :type Float%20%28double-precision%29) (TriggeredSeconds :type Float%20%28double-precision%29) (InputAction :type Input%20Action%20Object%20Reference :default "/Game/Inputs/IA_Look.IA_Look"))
  ;[0 0.8365 0.01879 0.5] Set angle of camera ball
  (bind _returnvalue (Actor|GetActorOfClass "/Game/BP/Ball/BP_Ball_Spawner.BP_Ball_Spawner_C"))
  (Variables|Default|SetBP_BallSpawner _returnvalue)
  (bind _returnvalue_2 (Actor|GetActorOfClass "/Game/BP/Ball/BP_Ball.BP_Ball_C"))
  (Variables|Default|SetBP_Ball _returnvalue_2)
  (Utilities|IsValid (Variables|Default|GetBP_BallSpawner)
    (:Is%20Valid
      (Default|BallRotation (Variables|Default|GetBP_Ball) (/ (Class|KismetMathLibrary|DegAtan2 (.x ActionValue) (.y ActionValue)) 5.0)))))

(event Input|EnhancedActionEvents|EnhancedInputActionIA_Pause
  (params (ActionValue :type Boolean) (ElapsedSeconds :type Float%20%28double-precision%29) (TriggeredSeconds :type Float%20%28double-precision%29) (InputAction :type Input%20Action%20Object%20Reference :default "/Game/Inputs/IA_Pause.IA_Pause"))
  (bind _returnvalue (Game|GetPlayerController 0))
  (:Started
    (if (not (Variables|Default|GetPaused))
      (bind _returnvalue_2 (UserInterface|CreateWidget "/Game/BP/Interface/WBP_Pause.WBP_Pause_C"))
      (UserInterface|Viewport|AddtoViewport _returnvalue_2 0)
      (Variables|/Script/Engine.PlayerController|SetbShowMouseCursor _returnvalue true)
      (Variables|Default|SetPaused true)
      (Game|SetGamePaused (Variables|Default|GetPaused))
      (Input|SetInputModeUIOnly _returnvalue 0 "DoNotLock" false))))

(event Input|EnhancedActionEvents|EnhancedInputActionIA_Move
  (params (ActionValue :type Float%20%28double-precision%29) (ElapsedSeconds :type Float%20%28double-precision%29) (TriggeredSeconds :type Float%20%28double-precision%29) (InputAction :type Input%20Action%20Object%20Reference :default "/Game/Inputs/IA_Move.IA_Move"))
  ;[0.03885 0.5971 0.7781 0.5] Paddle Povement
  (Transformation|AddLocalOffset (Variables|Default|GetPaddle) (Math|Vector|MakeVector 0.0 (* ActionValue (Variables|Default|GetPaddleSpeed)) 0.0) true false))

(event Input|EnhancedActionEvents|EnhancedInputActionIA_Pick
  (params (ActionValue :type Boolean) (ElapsedSeconds :type Float%20%28double-precision%29) (TriggeredSeconds :type Float%20%28double-precision%29) (InputAction :type Input%20Action%20Object%20Reference :default "/Game/Inputs/IA_Pick.IA_Pick"))
  (:Started
    (Variables|Default|SetState true)
    (Default|PressedE (Variables|Default|GetBP_Ball) (Variables|Default|GetState) :!label _label))
  (:Completed
    (Variables|Default|SetState false)
    (goto _label)))

(event EventBeginPlay
  (bind _returnvalue (Game|GetPlayerController 0))
  ;[1 0.000162 0.01892 0.5] Set UI and ball control
  (Input|SetInputModeGameOnly _returnvalue false)
  (Variables|/Script/Engine.PlayerController|SetbShowMouseCursor _returnvalue false)
  (bind _asplayer_controller (Utilities|Casting|CastToPlayerController (Pawn|GetController)))
  (Utilities|IsValid (PlayerController|LocalPlayerSubsystems|GetEnhancedInputLocalPlayerSubsystem _asplayer_controller)
    (:Is%20Valid
      (Input|AddMappingContext (PlayerController|LocalPlayerSubsystems|GetEnhancedInputLocalPlayerSubsystem _asplayer_controller) "/Game/Inputs/IMC_Paddle.IMC_Paddle" 0 "(bIgnoreAllPressedKeysUntilRelease=True,bForceImmediately=False,bNotifyUserSettings=False)")
      (bind _returnvalue_2 (Game|ConstructObjectfromClass "/Game/BP/Interface/WBP_HUD.WBP_HUD_C"))
      (bind _output_get (Variables|Default|SetPlayerHUD _returnvalue_2))
      (UserInterface|Viewport|AddtoViewport _output_get 0))))

(fn ConstructionScript)

(fn BallRotation
  (params (Rotation :type Float%20%28double-precision%29)))

(fn LevelChooser)