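; BP_Bricks is a breakable brick that loses a life each time a BP_Ball hits it and is destroyed at zero.
; UpdateBrickColor maps remaining lives to one of three materials, on construction and after non-fatal hits.
; On BeginPlay, a coin flip can spawn an actor above the brick, rerolling while no BP_Duck exists.
; The SpawnDuck function is an empty stub.
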(event OnComponentHit(Cube)
  (params (HitComponent :type Primitive%20Component%20Object%20Reference) (OtherActor :type Actor%20Object%20Reference) (OtherComp :type Primitive%20Component%20Object%20Reference) (NormalImpulse :type Vector :default "0, 0, 0") (Hit :type Hit%20Result%20Structure%20%28by%20ref%29))
  ;[0.9781 0.03921 0 0.5] Set brick life
  (Utilities|Casting|CastToBP_Ball OtherActor)
  (bind _result (Math|Integer|DecrementInt (Variables|Default|GetBrickLives))
    (:%20%20
      (if (== _result 0)
        (Actor|DestroyActor)
        (else
          (CallFunction|UpdateBrickColor))))))

(event EventBeginPlay
  (if (> (Math|Random|RandomIntegerinRange 1 2) 1) :!label _label
    (Game|SpawnActorfromClass "/Game/BP/OnMap/BP_Duck.BP_Duck_C" (Math|Transform|MakeTransform (+ (Transformation|GetActorLocation) "0.000000,0.000000,500.000000") "0, 0, 0" "1.000000,1.000000,1.000000") "AdjustIfPossibleButAlwaysSpawn" "MultiplyWithRoot" 0 0)
    (else
      (bind _returnvalue (Actor|GetActorOfClass "/Game/BP/OnMap/BP_Duck.BP_Duck_C"))
      (if (not (Utilities|IsValid _returnvalue))
        (goto _label)))))

(fn ConstructionScript
  (CallFunction|UpdateBrickColor))

(fn UpdateBrickColor
  (bind _cube (Variables|Default|GetCube))
  ;[0.8906 0 0 0.5] Change color by life of brick
  (switch int (Variables|Default|GetBrickLives)
    (:1
      (Rendering|Material|SetMaterial _cube 0 "/Game/Materials/Art/Bricks/M_State_3.M_State_3"))
    (:2
      (Rendering|Material|SetMaterial _cube 0 "/Game/Materials/Art/Bricks/M_State_2.M_State_2"))
    (:3
      (Rendering|Material|SetMaterial _cube 0 "/Game/Materials/Art/Bricks/M_State_1.M_State_1"))))

(fn SpawnDuck)